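; Player controller for the opening knight's dice battle, linking Battle events to the knight, camera and UI.
; BeginPlay sets the ortho camera, finds knight and enemy, and creates curtains, health bars, HUD and dice holder.
; Battle events refresh bars and dice, switch roll button mode by phase, and close curtains on victory.
; Player attacks start the knight's dash, then confirm the hit after a short delay.
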(event `self.Battle.OnStatsChanged`
  (params (Stats :type "OKStatsUI Structure"))
  (bind (_playerhp _playermaxhp _enemyhp _enemymaxhp) (break `OKStatsUI` Stats))
  (`KismetSystemLibrary.PrintString` "On Stats to Update Bars IS VALID ")
  (`/Engine/EditorBlueprintResources/StandardMacros.IsValid` (`self.HealthBarsRef`)
    (:`Is Valid`
      (`/Game/Images/UI/WBP_HealthBars.UpdateBars` (`self.HealthBarsRef`) _playerhp _playermaxhp _enemyhp _enemymaxhp))))

(event `InputAction|Attack`
  (params (Key :type "Key Structure"))
  (:`Pressed`
    (`/Game/Images/BP_Knight.StartAttachDash` (`self.KnightRef`) (`self.EnemyRef`))))

(event `self.ReceiveBeginPlay`
  (bind _battle (`self.Battle`))
  (bind _battle_2 (`self.Battle`))
  (bind _returnvalue (`|CreateWidget` "/Game/Images/Curtains/WBP_Curtains.WBP_Curtains_C"))
  (set `self.CurtainsRef` _returnvalue)
  (`UserWidget.AddToViewport` _returnvalue 500)
  (`/Game/Images/Curtains/WBP_Curtains.OpenCurtains` _returnvalue)
  (bind _returnvalue_2 (`|CreateWidget` "/Game/Images/UI/WBP_HealthBars.WBP_HealthBars_C"))
  (bind _output_get (set `self.HealthBarsRef` _returnvalue_2))
  (`UserWidget.AddToViewport` _output_get 0)
  (`/Game/Images/UI/WBP_HealthBars.UpdateBars` (`self.HealthBarsRef`) (`OpeningKnightBattleComponent.GetPlayerHP` _battle) (`OpeningKnightBattleComponent.GetPlayerMaxHP` _battle) (`OpeningKnightBattleComponent.GetEnemyHP` _battle) (`OpeningKnightBattleComponent.GetEnemyMaxHP` _battle))
  (add `OpeningKnightBattleComponent.OnPhaseChanged` (`self.Battle`) (delegate `OnPhaseChanged_Event`))
  (add `OpeningKnightBattleComponent.OnPlayerAttackStarted` _battle_2 (delegate `OnPlayerAttackStarted_Event`))
  (set `self.HeldDice` (`|MakeArray` false false false false false false))
  (`|ExecutionSequence`
    (:`then_0`
      (bind _outactors (`GameplayStatics.GetAllActorsOfClass` "/Game/BP_OrthoCamera.BP_OrthoCamera_C"))
      (`self.SetViewTargetWithBlend` (`|GetArrayItem` _outactors)))
    (:`then_1`
      (bind _outactors_2 (`GameplayStatics.GetAllActorsOfClass` "/Game/Images/BP_Knight.BP_Knight_C"))
      (set `self.KnightRef` (`|GetArrayItem` _outactors_2))
      (bind _outactors_3 (`GameplayStatics.GetAllActorsOfClass` "/Game/Images/Enemies/BP_Enemy.BP_Enemy_C"))
      (set `self.EnemyRef` (`|GetArrayItem` _outactors_3)))
    (:`then_2`
      (bind _returnvalue_3 (`|CreateWidget` "/Game/Images/UI/WBP_Play_BillHUD.WBP_Play_BillHUD_C" self))
      (set `self.PlayBillHUDRef` _returnvalue_3)
      (`/Game/Images/UI/WBP_Play_BillHUD.SetRollButtonMode` (`self.PlayBillHUDRef`) false)
      (`UserWidget.AddToViewport` (`self.PlayBillHUDRef`) 0)
      (bind _returnvalue_4 (`|CreateWidget` "/Game/Images/UI/WBP_Dice_Holder.WBP_Dice_Holder_C" self))
      (set `self.DiceHolderRef` _returnvalue_4)
      (`UserWidget.AddToViewport` (`self.DiceHolderRef`) 0)
      (set `self.bShowMouseCursor` true)
      (add `OpeningKnightBattleComponent.OnDiceChanged` _battle_2 (delegate `OnDiceChanged_Event`))
      (`WidgetBlueprintLibrary.SetInputMode_GameAndUIEx` self (`self.PlayBillHUDRef`)))))

(event `OnPhaseChanged_Event`
  (params (Phase :type "EOKTurnPhase Enum" :default "WaitingForRoll"))
  (bind _playbillhudref (`self.PlayBillHUDRef`))
  (switch `EOKTurnPhase` Phase
    (:`WaitingForRoll`
      (`/Game/Images/UI/WBP_Play_BillHUD.SetRollButtonMode` _playbillhudref false :!label _label))
    (:`PlayerSelecting`
      (`/Game/Images/UI/WBP_Play_BillHUD.SetRollButtonMode` _playbillhudref true))
    (:`AwaitingPlayerHitConfirm`
      (goto _label))
    (:`EnemyTurn`
      (goto _label))
    (:`Victory`
      (`KismetSystemLibrary.PrintString` "VICTORY PIN FIRED")
      (`/Game/Images/Curtains/WBP_Curtains.CloseCurtains` (`self.CurtainsRef`))
      (goto _label))
    (:`Defeat`
      (goto _label))))

(event `OnPlayerAttackStarted_Event`
  (params (PendingDamage :type Integer) (DebugText :type String))
  (`KismetSystemLibrary.PrintString` DebugText)
  (`/Game/Images/BP_Knight.StartAttachDash` (`self.KnightRef`) (`self.EnemyRef`))
  (`KismetSystemLibrary.Delay` 0.2)
  (`self.ConfirmPlayerHit`))

(event `OnDiceChanged_Event`
  (params (Dice :type "Array of OKDieUI Structure (by ref)"))
  (set `self.DiceState` Dice)
  (`/Game/Images/UI/WBP_Dice_Holder.UpdateDice` (`self.DiceHolderRef`) (`self.DiceState`) (`self.HeldDice`)))

(fn `OnDiceClicked`
  (params (Index :type Integer))
  (if (< Index (`KismetArrayLibrary.Array_Length` (`self.DiceState`)))
    (`KismetArrayLibrary.Array_Set` (`self.HeldDice`) Index)
    (`/Game/Images/UI/WBP_Dice_Holder.UpdateDice` (`self.DiceHolderRef`) (`self.DiceState`) (`self.HeldDice`))))

(fn `UserConstructionScript`)