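; BP_Knight is a knight actor that performs a melee dash attack toward a target and back to its starting spot.
; StartAttachDash stops short of the target along X only and scales play rate by distance and dash speed.
; A timeline lerps the location out, then reverses home; its Knight event enables the hitbox and flashes the shared hit-cloud effect there, cached on BeginPlay.
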(event `self.ReceiveBeginPlay`
  (cast `OpeningKnightPlayerController` (`GameplayStatics.GetPlayerController` 0))
  (bind _returnvalue (`OpeningKnightPlayerController.GetHitCloudInWorld`))
  (set `self.HitCloudRef` _returnvalue))

(event `Dash_Play`
  (bind _knighthitbox (`self.KnightHitBox`))
  (`TimelineComponent.SetPlayRate` (`self.TL_AttackDash`) (`self.DashPlayRate`))
  (bind (_direction _alpha) (`Timeline|TL_AttackDash` :!via `PlayFromStart` :!label _label)
    (:`Update`
      (`self.K2_SetActorLocation` (`KismetMathLibrary.VLerp` (`self.HomeLocation`) (`self.DashTargetLocation`) _alpha)))
    (:`Finished`
      (if (`self.bDashReturning`)
        (`self.K2_SetActorLocation` (`self.HomeLocation`))
        (set `self.bIsDashing` false)
        (set `self.bDashReturning` false)
        (else
          (set `self.bDashReturning` true)
          (goto _label :!via `Reverse`))))
    (:`EventKnight`
      (`PrimitiveComponent.SetCollisionEnabled` _knighthitbox "QueryOnly")
      (bind _asbp_hit_cloud_fx (cast `/Game/Images/BP_HitCloudFX` (`self.HitCloudRef`)))
      (`self.K2_SetActorLocation` _asbp_hit_cloud_fx (`SceneComponent.K2_GetComponentLocation` _knighthitbox) false false)
      (`/Game/Images/BP_HitCloudFX.Flash` _asbp_hit_cloud_fx))))

(fn `StartAttachDash`
  (params (TargetActor :type "Actor Object Reference"))
  (if (not (`self.bIsDashing`))
    (set `self.bIsDashing` true)
    (set `self.bDashReturning` false)
    (set `self.HomeLocation` (`self.K2_GetActorLocation`))
    (set `self.DashTargetLocation` (`KismetMathLibrary.MakeVector` (- (.x (`self.K2_GetActorLocation` TargetActor)) (`self.StopShortDistance`)) (.y (`self.HomeLocation`)) (.z (`self.HomeLocation`))))
    (set `self.DashPlayRate` (/ 1.0 (`KismetMathLibrary.FMax` (/ (`KismetMathLibrary.Vector_Distance` (`self.HomeLocation`) (`self.DashTargetLocation`)) (`self.DashSpeed`)) 0.05)))
    (`self.Dash_Play`)))

(fn `TargetActor`
  (if (`self.bIsDashing`)
    _))

(fn `UserConstructionScript`)