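; BP_HitCloudFX is a reusable effect actor that briefly shows a cloud sprite, apparently as hit feedback.
; PlayAtLocation moves the actor to a world location, unhides CloudSprite, waits for FXDuration, then hides it again.
; Flash does the same show and hide in place with a short fixed delay.
; The actor toggles visibility rather than spawning or destroying anything, and has no active Tick or construction logic.
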(event `PlayAtLocation`
  (params (WorldLocation :type "Vector Structure"))
  (`self.K2_SetActorLocation` WorldLocation)
  (`SceneComponent.SetHiddenInGame` (`self.CloudSprite`) false false)
  (`KismetSystemLibrary.Delay` (`self.FXDuration`))
  (`SceneComponent.SetHiddenInGame` (`self.CloudSprite`) true false))

(event `Flash`
  (`SceneComponent.SetHiddenInGame` (`self.CloudSprite`) false false)
  (`KismetSystemLibrary.Delay` 0.18)
  (`SceneComponent.SetHiddenInGame` (`self.CloudSprite`) true false))

(fn `UserConstructionScript`)