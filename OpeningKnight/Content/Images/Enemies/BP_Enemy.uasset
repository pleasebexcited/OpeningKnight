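; BP_Enemy is a battle enemy that performs turn-based dash attacks against BP_Knight and plays knockback reactions.
; StartAttack drives a speed-scaled timeline dash along X, stopping short of the target, then reversing home to end the enemy turn.
; A timeline event enables the hitbox and flashes a hit cloud; overlap confirms one hit through the controller's Battle.
; Blocking freezes the dash by zeroing its play rate.
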(event `self.AttackHitBox.OnComponentBeginOverlap`
  (params (OverlappedComponent :type "PrimitiveComponent Object Reference") (OtherActor :type "Actor Object Reference") (OtherComp :type "PrimitiveComponent Object Reference") (OtherBodyIndex :type Integer) (bFromSweep :type Boolean) (SweepResult :type "HitResult Structure (by ref)"))
  (cast `/Game/Images/BP_Knight` OtherActor)
  (if (and (`self.bIsAttacking`) (not (`self.bHasAppliedDamageThisAttack`)))
    (bind _asbp_opening_knight_player_controller (cast `/Game/BP_OpeningKnightPlayerController` (`GameplayStatics.GetPlayerController` 0)))
    (`OpeningKnightBattleComponent.ConfirmEnemyHit` (`OpeningKnightPlayerController.Battle` _asbp_opening_knight_player_controller))
    (set `self.bHasAppliedDamageThisAttack` true)))

(event `Attack_Play`
  (bind _attackhitbox (`self.AttackHitBox`))
  (bind _attackhomelocation (`self.AttackHomeLocation`))
  (`TimelineComponent.SetPlayRate` (`self.TL_AttackDash`) (`self.AttackPlayRate`))
  (bind (_direction _alpha) (`Timeline|TL_AttackDash` :!via `PlayFromStart`)
    (:`Update`
      (`self.K2_SetActorLocation` (`KismetMathLibrary.VLerp` _attackhomelocation (`self.AttackTargetLocation`) _alpha)))
    (:`Finished`
      (if (`self.bAttackReturning`)
        (`self.K2_SetActorLocation` _attackhomelocation)
        (set `self.bIsAttacking` false)
        (set `self.bAttackReturning` false)
        (`PrimitiveComponent.SetCollisionEnabled` (`self.AttackHitBox`) "NoCollision")
        (set `self.bHasAppliedDamageThisAttack` false)
        (bind _asbp_opening_knight_player_controller (cast `/Game/BP_OpeningKnightPlayerController` (`GameplayStatics.GetPlayerController` 0)))
        (`OpeningKnightBattleComponent.FinishEnemyTurn` (`OpeningKnightPlayerController.Battle` _asbp_opening_knight_player_controller))
        (else
          (set `self.bAttackReturning` true)
          (`TimelineComponent.ReverseFromEnd` (`self.TL_AttackDash`)))))
    (:`HitCloudEvent`
      (`PrimitiveComponent.SetCollisionEnabled` _attackhitbox "QueryOnly")
      (`self.K2_SetActorLocation` (`self.HitCloudRef`) (`SceneComponent.K2_GetComponentLocation` _attackhitbox) false false)
      (`/Game/Images/BP_HitCloudFX.Flash` (`self.HitCloudRef`)))))

(event `self.ReceiveBeginPlay`
  (`PrimitiveComponent.SetCollisionEnabled` (`self.AttackHitBox`) "NoCollision"))

(event `PlayHitReact`
  (params (AttackerActor :type "Actor Object Reference"))
  (if (not (`self.bIsHitReacting`))
    (`/Game/Images/BP_HitCloudFX.Flash` (`self.HitCloudRef`))
    (set `self.bIsHitReacting` true)
    (set `self.EnemyHomeLocation` (`self.K2_GetActorLocation`))
    (set `self.EnemyBackLocation` (`KismetMathLibrary.MakeVector` (+ (.x (`self.EnemyHomeLocation`)) (`self.KnockbackDistance`)) (.y (`self.EnemyHomeLocation`)) (.z (`self.EnemyHomeLocation`))))
    (bind (_direction _alpha) (`Timeline|TL_HitReact` :!via `PlayFromStart`)
      (:`Update`
        (`self.K2_SetActorLocation` (`KismetMathLibrary.VLerp` (`self.EnemyHomeLocation`) (`self.EnemyBackLocation`) _alpha)))
      (:`Finished`
        (`self.K2_SetActorLocation` (`self.EnemyHomeLocation`))
        (set `self.bIsHitReacting` true)
        (`self.K2_SetActorLocation` (`self.EnemyHomeLocation`))))))

(event `self.HitTrigger.OnComponentEndOverlap`
  (params (OverlappedComponent :type "PrimitiveComponent Object Reference") (OtherActor :type "Actor Object Reference") (OtherComp :type "PrimitiveComponent Object Reference") (OtherBodyIndex :type Integer))
  (goto _label :!via `Reset`))

(event `self.HitTrigger.OnComponentBeginOverlap`
  (params (OverlappedComponent :type "PrimitiveComponent Object Reference") (OtherActor :type "Actor Object Reference") (OtherComp :type "PrimitiveComponent Object Reference") (OtherBodyIndex :type Integer) (bFromSweep :type Boolean) (SweepResult :type "HitResult Structure (by ref)"))
  (cast `/Game/Images/BP_Knight` OtherActor)
  (`/Engine/EditorBlueprintResources/StandardMacros.DoOnce` false :!label _label
    (:`Completed`
      (`self.PlayHitReact` OtherActor))))

(event `Freeze For Block`
  (`TimelineComponent.SetPlayRate` (`self.TL_AttackDash`) 0.0))

(event `Unfreeze From Block`
  (`TimelineComponent.SetPlayRate` (`self.TL_AttackDash`) (`self.AttackPlayRate`)))

(fn `ReturnToPosition`
  (`TimelineComponent.Stop` (`self.TL_AttackDash`))
  (`self.K2_SetActorLocation` (`self.AttackHomeLocation`))
  (set `self.bIsAttacking` false))

(fn `StartAttack`
  (params (`Target Actor` :type "Actor Object Reference"))
  (if (not (`self.bIsAttacking`))
    (set `self.bIsAttacking` true)
    (`PrimitiveComponent.SetCollisionEnabled` (`self.AttackHitBox`) "NoCollision")
    (set `self.bAttackReturning` false)
    (set `self.AttackHomeLocation` (`self.K2_GetActorLocation`))
    (set `self.AttackTargetLocation` (`KismetMathLibrary.MakeVector` (+ (.x (`self.K2_GetActorLocation` `Target Actor`)) (`self.StopShortDistance`)) (.y (`self.AttackHomeLocation`)) (.z (`self.AttackHomeLocation`))))
    (set `self.AttackPlayRate` (/ 1.0 (`KismetMathLibrary.FMax` (/ (`KismetMathLibrary.Vector_Distance` (`self.AttackHomeLocation`) (`self.AttackTargetLocation`)) (`self.AttackSpeed`)) 0.05)))
    (`self.Attack_Play`)))

(fn `UserConstructionScript`)